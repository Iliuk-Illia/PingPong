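; Pong-style ball that launches in a random Y direction and moves by feeding its Velocity to FloatingPawnMovement every tick.
; Overlaps flip X on walls, while character hits flip Y, raise max speed and add sideways spin from stored energy or character velocity, clearing that energy.
; Goal zones increment a GameMode score, spawn a replacement ball handed to the EnemyCharacter, and destroy this one.
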(event `self.ReceiveBeginPlay`
  (set `self.Velocity` (`KismetMathLibrary.MakeVector` 0.0 (`KismetMathLibrary.SelectFloat` -1.0 1.0 (`KismetMathLibrary.RandomBool`)))))

(event `self.ReceiveTick`
  (params (DeltaSeconds :type "Float (single-precision)"))
  (`PawnMovementComponent.AddInputVector` (`self.FloatingPawnMovement`) (`self.Velocity`) false))

(event `self.Sphere1.OnComponentBeginOverlap`
  (params (OverlappedComponent :type "PrimitiveComponent Object Reference") (OtherActor :type "Actor Object Reference") (OtherComp :type "PrimitiveComponent Object Reference") (OtherBodyIndex :type Integer) (bFromSweep :type Boolean) (SweepResult :type "HitResult Structure (by ref)"))
  (bind (_velocity_x _velocity_y _velocity_z) (`KismetMathLibrary.BreakVector` (`self.Velocity`)))
  (bind (_velocity_x_2 _velocity_y_2 _velocity_z_2) (`KismetMathLibrary.BreakVector` (`self.Velocity`)))
  (bind _floatingpawnmovement (`self.FloatingPawnMovement`))
  (cast `/Game/Blueprints/BP_Wall` OtherActor
    (:`then`
      (`GameplayStatics.PlaySound2D` "/Game/Audio/ping_pong_8bit_plop.ping_pong_8bit_plop" 1.0 1.0 0.0 null null)
      (set `self.Velocity` (`KismetMathLibrary.MakeVector` (* _velocity_x_2 -1.0) _velocity_y_2 _velocity_z_2)))
    (:`CastFailed`
      (bind _asplayer_character (cast `PlayerCharacter` OtherActor)
        (:`then`
          (`GameplayStatics.PlaySound2D` "/Game/Audio/ping_pong_8bit_beeep.ping_pong_8bit_beeep" 1.0 1.0 0.0 null null)
          (cast `BoxComponent` OtherComp)
          (bind _returnvalue_x (`KismetMathLibrary.BreakVector` (`self.GetVelocity` _asplayer_character)))
          (set `self.Velocity` (`KismetMathLibrary.MakeVector` (+ _velocity_x (select `bool` (`PlayerCharacter.Energy` _asplayer_character) :`false` (/ _returnvalue_x (`MovementComponent.GetMaxSpeed` (`self.GetMovementComponent` _asplayer_character))) :`true` (`PlayerCharacter.VelocityToEnergy` _asplayer_character) :!type "Float (double-precision)")) (* _velocity_y -1.0) _velocity_z))
          (set `FloatingPawnMovement.MaxSpeed` (* (`MovementComponent.GetMaxSpeed` _floatingpawnmovement) (`self.SpeedMultiplier`)) _floatingpawnmovement)
          (set `PlayerCharacter.Energy` false _asplayer_character)
          (`PrimitiveComponent.SetMaterial` (`PlayerCharacter.StaticMesh` _asplayer_character) 0 "/Engine/BasicShapes/BasicShapeMaterial.BasicShapeMaterial"))
        (:`CastFailed`
          (bind _asbp_goal_zone (cast `/Game/Blueprints/BP_GoalZone` OtherActor))
          (`self.Goal` (`/Game/Blueprints/BP_GoalZone.PlayerTargetGoal` _asbp_goal_zone))
          (`GameplayStatics.PlaySound2D` "/Game/Audio/Goal.Goal" 1.0 1.0 0.0 null null)
          (`self.K2_DestroyActor`))))))

(event `Goal`
  (params (PlayerGoal :type Boolean))
  (`|ExecutionSequence`
    (:`then_0`
      (bind _returnvalue (`|SpawnActorFromClass` "BP_Ball_C" (`KismetMathLibrary.MakeTransform` (0.0 0.0 40.0)) "Undefined" "MultiplyWithRoot" null null))
      (bind _returnvalue_2 (`GameplayStatics.GetActorOfClass` "/Game/Blueprints/EnemyCharacter.EnemyCharacter_C"))
      (set `/Game/Blueprints/EnemyCharacter.Ball` _returnvalue _returnvalue_2))
    (:`then_1`
      (bind _asbp_my_game_mode_base (cast `/Game/Blueprints/BP_MyGameModeBase` (`GameplayStatics.GetGameMode`)))
      (`/Engine/EditorBlueprintResources/StandardMacros.IncrementInt` (select `int` (`KismetMathLibrary.Conv_BoolToInt` PlayerGoal) :`0` (`/Game/Blueprints/BP_MyGameModeBase.EnemyScore` _asbp_my_game_mode_base) :`1` (`/Game/Blueprints/BP_MyGameModeBase.PlayerScore` _asbp_my_game_mode_base))))))

(fn `UserConstructionScript`)