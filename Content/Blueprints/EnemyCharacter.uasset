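; Enemy character that continuously chases the ball along the world X axis.
; BeginPlay finds the BP_Ball actor in the level and caches it.
; Each Tick compares X positions and adds full movement input toward the ball's side, with no dead zone or validity check on the reference.
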(event `self.ReceiveBeginPlay`
  (bind _returnvalue (`GameplayStatics.GetActorOfClass` "/Game/Blueprints/BP_Ball.BP_Ball_C"))
  (set `self.Ball` _returnvalue))

(event `self.ReceiveTick`
  (params (DeltaSeconds :type "Float (single-precision)"))
  (bind _returnvalue_x (`KismetMathLibrary.BreakVector` (`self.K2_GetActorLocation`)))
  (bind _returnvalue_x_2 (`KismetMathLibrary.BreakVector` (`self.K2_GetActorLocation` (`self.Ball`))))
  (`self.AddMovementInput` (`KismetMathLibrary.MakeVector` (select `bool` (> (- _returnvalue_x_2 _returnvalue_x) 0.0) :`false` -1.0 :`true` 1.0))))

(fn `UserConstructionScript`
  (`parent.UserConstructionScript`))